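; BP_EnemyAI is an enemy pawn that reacts to seeing another pawn by running to a random spot on the navmesh.
; PawnSensing sight sets IsSeeingPlayer and calls RunFromPlayer, which issues AI MoveTo within a very large radius, without steering away from the player.
; A FollowPlayer event can chase the player character, but nothing here calls it.
; Noise hearing is unimplemented, and IsSeeingPlayer is never read or cleared here.
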(event `self.PawnSensing.OnSeePawn`
  (params (Pawn :type "Pawn Object Reference"))
  (set `self.isSeeingPlayer` true)
  (`self.RunFromPlayer`))

(event `self.PawnSensing.OnHearNoise`
  (params (Instigator :type "Pawn Object Reference") (Location :type "Vector Structure (by ref)") (Volume :type "Float (single-precision)")))

(event `RunFromPlayer`
  (if true
    (bind _randomlocation (`NavigationSystemV1.K2_GetRandomLocationInNavigableRadius` (`CharacterMovementComponent.GetLastUpdateLocation` (`self.CharacterMovement`)) 50000.0 null null))
    (`|AIMoveTo` self _randomlocation null)))

(event `FollowPlayer`
  (if true
    (`|AIMoveTo` self (0.0 0.0 0.0) (`GameplayStatics.GetPlayerCharacter` 0) 70.0)))

(fn `UserConstructionScript`)